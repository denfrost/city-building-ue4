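; City game state that runs the simulated clock and calendar and displays them on the main HUD.
; Each tick advances the clock by a speed-scaled time unit, splits it into seconds, minutes and hours, and feeds day ticks into the calendar.
; Calendar rolls days into months and updates the HUD date only when the month exceeds 12, without resetting it.
; Speed changes rescale the time unit and are broadcast; SetClock and SetCalendar are empty stubs.
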(event EventBeginPlay
  (bind _ascity_camera_controller (Utilities|Casting|CastToCityCameraController (Game|GetPlayerController 0)))
  (Variables|Reference|SetControllerRef _ascity_camera_controller)
  (Variables|Clock|SetClock (+ (Math|Conversions|ToFloat(Integer) (Variables|Clock|GetHours)) (Math|Conversions|ToFloat(Integer) (Variables|Clock|GetMinutes)) (Math|Conversions|ToFloat(Integer) (Variables|Clock|GetSeconds))))
  (Variables|Calendar|SetGameDate (Utilities|Array|MakeArray (Variables|Calendar|GetDay) (Variables|Calendar|GetMonth) (Variables|Calendar|GetYear)))
  (Variables|Reference|SetMainUIRef (Variables|/Game/CityGame/Blueprints/CityCameraController.CityCameraController_C|GetMainHUDRef (Variables|Reference|GetControllerRef)))
  (Variables|Default|SetTimeUnit (Variables|Default|GetDefaultGameSpeed)))

(event EventUpdateGameStateSpeed
  (params (Multiplier :type Float%20%28single-precision%29))
  (bind _output_get (Variables|Default|SetTimeUnit (* Multiplier (Variables|Default|GetDefaultGameSpeed))))
  (Default|CallUpdateGameSpeed _output_get))

(event EventTick
  (params (DeltaSeconds :type Float%20%28single-precision%29))
  (bind (_clockout _daytick) (CallFunction|SetClockWork DeltaSeconds (Variables|Default|GetTimeUnit) (Variables|Clock|GetClock)))
  (Variables|Clock|SetClock _clockout)
  (Variables|Calendar|SetDayTick _daytick)
  (CallFunction|ClockWork)
  (CallFunction|Calendar))

(fn ConstructionScript)

(fn ClockWork
  (bind _clock (Variables|Clock|GetClock))
  (bind _returnvalue (* _clock 3.6e+03))
  (bind (_remainder _returnvalue_2) (Math|Float|Division(WholeandRemainder) _returnvalue 0.0))
  (bind _returnvalue_3 (Math|Conversions|ToFloat(Integer) _returnvalue_2))
  (bind (_remainder_2 _returnvalue_4) (Math|Float|Division(WholeandRemainder) _returnvalue_3 6e+01))
  (Variables|Clock|SetSeconds (Math|Float|Floor _remainder))
  (Variables|Clock|SetMinutes (Math|Float|Floor _remainder_2))
  (Variables|Clock|SetHours (Math|Float|Floor (.Remainder (Math|Float|Division(WholeandRemainder) (Math|Conversions|ToFloat(Integer) _returnvalue_4) 24.0))))
  (bind _output_get (Variables|Clock|SetGameTime (Utilities|Array|MakeArray (Variables|Clock|GetSeconds) (Variables|Clock|GetMinutes) (Variables|Clock|GetHours))))
  (Class|HUDI|SetClock(Message) (Variables|Reference|GetMainUIRef) _output_get))

(fn Calendar
  (bind _output_get (Variables|Calendar|SetDay (+ (Variables|Calendar|GetDayTick) (Variables|Calendar|GetDay))))
  (if (> _output_get (Class|KismetMathLibrary|DaysinMonth (Variables|Calendar|GetYear) (Variables|Calendar|GetMonth)))
    (Variables|Calendar|SetDay 1)
    (Variables|Calendar|SetMonth (+ (Variables|Calendar|GetMonth) 1)))
  (if (> (Variables|Calendar|GetMonth) 12)
    (Variables|Calendar|SetYear (+ (Variables|Calendar|GetYear) 1))
    (bind _output_get_2 (Variables|Calendar|SetGameDate (Utilities|Array|MakeArray (Variables|Calendar|GetDay) (Variables|Calendar|GetMonth) (Variables|Calendar|GetYear))))
    (Class|HUDI|SetCalendar(Message) (Variables|Reference|GetMainUIRef) _output_get_2)))

(fn SetCalendar
  (params (Day :type Array%20of%20Integers))
  (return 0))

(fn SetClock
  (params (Time :type Array%20of%20Integers))
  (return 0))