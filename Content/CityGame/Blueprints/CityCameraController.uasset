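; Player controller for the city game that drives the MainCamera pawn and creates the main HUD with the game state.
; Input zooms the spring arm within limits and moves the pawn along its local axes at a speed based on clamped arm length.
; Holding Pan opens gates that let mouse movement yaw and pitch the pawn, with pitch clamped.
; Sideways movement forces a fixed height, and separate inputs reset zoom and pitch.
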(event EventBeginPlay
  ;[1 1 1] Begin Play
  (Utilities|FlowControl|Sequence
    (:then_0
      (Utilities|CastReference))
    (:then_1
      (Input|SetInputModeGameandUI self 0 "LockOnCapture" true)
      (Utilities|CreateHUD)
      (UserInterface|Viewport|AddtoViewport (Variables|Reference|GetMainHUDRef) 0))))

(event Input|ActionEvents|InputActionZoomIn
  (params (Key :type Key%20Structure :default "None"))
  (bind _camerapawnref (Variables|Reference|GetCameraPawnRef))
  (bind _springarm (Variables|/Game/CityGame/Blueprints/MainCamera.MainCamera_C|GetSpringArm _camerapawnref))
  ;[1 1 1] Camera Zoom
  (:Pressed
    (Variables|/Script/Engine.SpringArmComponent|SetTargetArmLength _springarm (Math|Float|Clamp(Float) (- (Variables|/Script/Engine.SpringArmComponent|GetTargetArmLength _springarm) (Variables|CameraSettings|GetZoomSensitivity)) (Variables|CAmeraSettings|GetMinArmDistance) (Variables|CAmeraSettings|GetMaxArmDistance)))))

(event Input|ActionEvents|InputActionZoomOut
  (params (Key :type Key%20Structure :default "None"))
  (bind _camerapawnref (Variables|Reference|GetCameraPawnRef))
  (bind _springarm (Variables|/Game/CityGame/Blueprints/MainCamera.MainCamera_C|GetSpringArm _camerapawnref))
  ;[1 1 1] Camera Zoom
  (:Pressed
    (Variables|/Script/Engine.SpringArmComponent|SetTargetArmLength _springarm (Math|Float|Clamp(Float) (+ (Variables|/Script/Engine.SpringArmComponent|GetTargetArmLength _springarm) (Variables|CameraSettings|GetZoomSensitivity)) (Variables|CAmeraSettings|GetMinArmDistance) (Variables|CAmeraSettings|GetMaxArmDistance)))))

(event Input|ActionEvents|InputActionZoomReset
  (params (Key :type Key%20Structure :default "None"))
  ;[1 1 1] Reset Zoom
  (:Pressed
    (Variables|/Script/Engine.SpringArmComponent|SetTargetArmLength (Variables|/Game/CityGame/Blueprints/MainCamera.MainCamera_C|GetSpringArm (Variables|Reference|GetCameraPawnRef)) (Variables|CameraSettings|GetDefaultArmDistance))))

(event Input|ActionEvents|InputActionPan
  (params (Key :type Key%20Structure :default "None"))
  (bind _camerapawnref (Variables|Reference|GetCameraPawnRef))
  (bind _returnvalue (Transformation|GetActorRotation _camerapawnref))
  (bind (_roll _pitch _yaw) (Math|Rotator|BreakRotator _returnvalue))
  ;[1 1 1] Pan X
  (:Pressed
    (Variables|Booleans|SetDisabeCamNav false)
    (Utilities|FlowControl|Gate true) ; enters at Open
  )
  (:Released
    (Variables|Booleans|SetDisabeCamNav false)
    (Utilities|FlowControl|Gate true) ; enters at Close
  ))

(event Input|ActionEvents|InputActionPan
  (params (Key :type Key%20Structure :default "None"))
  (bind _camerapawnref (Variables|Reference|GetCameraPawnRef))
  (bind _returnvalue (Transformation|GetActorRotation _camerapawnref))
  (bind (_roll _pitch _yaw) (Math|Rotator|BreakRotator _returnvalue))
  ;[1 1 1] Pan Y
  (:Pressed
    (Variables|Booleans|SetDisabeCamNav false)
    (Utilities|FlowControl|Gate true) ; enters at Open
  )
  (:Released
    (Variables|Booleans|SetDisabeCamNav false)
    (Utilities|FlowControl|Gate true) ; enters at Close
  ))

(event Input|ActionEvents|InputActionResetPan
  (params (Key :type Key%20Structure :default "None"))
  (bind _camerapawnref (Variables|Reference|GetCameraPawnRef))
  (bind _returnvalue (Transformation|GetActorRotation _camerapawnref))
  (bind (_roll _pitch _yaw) (Math|Rotator|BreakRotator _returnvalue))
  ;[1 1 1] Pan Reset
  (:Pressed
    (Transformation|SetActorRotation (Variables|Reference|GetCameraPawnRef) (Math|Rotator|MakeRotator _roll 0.0 _yaw))))

(event Input|AxisEvents|InputAxisMoveForward
  (params (AxisValue :type Float%20%28single-precision%29))
  ;[1 1 1] Move Forward
  (if (not (Variables|Booleans|GetDisabeCamNav))
    (Transformation|SetActorTransform (Variables|Reference|GetCameraPawnRef) (Utilities|MoveX (CallFunction|MoveSpeedCalc) 1.0 AxisValue (Variables|Reference|GetCameraPawnRef)))))

(event Input|AxisEvents|InputAxisMoveRight
  (params (AxisValue :type Float%20%28single-precision%29))
  (bind _movesensitivity (CallFunction|MoveSpeedCalc))
  (bind _camerapawnref (Variables|Reference|GetCameraPawnRef))
  (bind _transform (Utilities|MoveY _movesensitivity 1.0 AxisValue _camerapawnref))
  (bind (_location _rotation _scale) (Math|Transform|BreakTransform _transform))
  (bind (_x _y) (Math|Vector|BreakVector _location))
  ;[1 1 1] Move Right-Left
  (if (not (Variables|Booleans|GetDisabeCamNav))
    (Transformation|SetActorTransform (Variables|Reference|GetCameraPawnRef) (Math|Transform|MakeTransform (Math|Vector|MakeVector _x _y 5e+02) _rotation _scale))))

(event Input|MouseEvents|MouseX
  (params (AxisValue :type Float%20%28single-precision%29))
  (bind _camerapawnref (Variables|Reference|GetCameraPawnRef))
  (bind _returnvalue (Transformation|GetActorRotation _camerapawnref))
  (bind (_roll _pitch _yaw) (Math|Rotator|BreakRotator _returnvalue))
  ;[1 1 1] Pan X
  (Utilities|FlowControl|Gate true
    (:Exit
      (Transformation|SetActorRotation (Variables|Reference|GetCameraPawnRef) (Math|Rotator|MakeRotator _roll _pitch (+ _yaw (* AxisValue (Variables|CameraSettings|GetPanSensitivity))))))))

(event Input|MouseEvents|MouseY
  (params (AxisValue :type Float%20%28single-precision%29))
  (bind _camerapawnref (Variables|Reference|GetCameraPawnRef))
  (bind _returnvalue (Transformation|GetActorRotation _camerapawnref))
  (bind (_roll _pitch _yaw) (Math|Rotator|BreakRotator _returnvalue))
  ;[1 1 1] Pan Y
  (Utilities|FlowControl|Gate true
    (:Exit
      (Transformation|SetActorRotation (Variables|Reference|GetCameraPawnRef) (Math|Rotator|MakeRotator _roll (Math|Float|Clamp(Float) (+ _pitch (* AxisValue (Variables|CameraSettings|GetPanSensitivity))) -5.0 75.0) _yaw)))))

(fn ConstructionScript)

(fn MoveSpeedCalc
  (return (Math|Float|Clamp(Float) (/ (Variables|/Script/Engine.SpringArmComponent|GetTargetArmLength (Variables|/Game/CityGame/Blueprints/MainCamera.MainCamera_C|GetSpringArm (Variables|Reference|GetCameraPawnRef))) 1.0) 5.0 2e+01)))